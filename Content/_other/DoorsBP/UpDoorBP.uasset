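; Door Blueprint that slides DoorDown up when something overlaps its Box trigger and lowers it when the overlap ends.
; Two timelines lerp the mesh's relative location from its current position toward the DoorUp or DoorDownP component locations.
; Two DoOnce gates sequence the motion: the finished opening resets the closing gate, and the finished closing resets the opening gate.
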(event `self.Box.OnComponentBeginOverlap`
  (params (OverlappedComponent :type "PrimitiveComponent Object Reference") (OtherActor :type "Actor Object Reference") (OtherComp :type "PrimitiveComponent Object Reference") (OtherBodyIndex :type Integer) (bFromSweep :type Boolean) (SweepResult :type "HitResult Structure (by ref)"))
  (`/Engine/EditorBlueprintResources/StandardMacros.DoOnce` false :!label _label
    (:`Completed`
      (bind (_direction _newtrack_0) (`Timeline|Timeline_0` :!via `PlayFromStart`)
        (:`Update`
          (`SceneComponent.K2_SetRelativeLocation` (`self.DoorDown`) (`KismetMathLibrary.VLerp` (`SceneComponent.RelativeLocation` (`self.DoorDown`)) (`SceneComponent.RelativeLocation` (`self.DoorUp`)) _newtrack_0) false false))
        (:`Finished`
          (goto _label_2 :!via `Reset`))))))

(event `self.Box.OnComponentEndOverlap`
  (params (OverlappedComponent :type "PrimitiveComponent Object Reference") (OtherActor :type "Actor Object Reference") (OtherComp :type "PrimitiveComponent Object Reference") (OtherBodyIndex :type Integer))
  (`/Engine/EditorBlueprintResources/StandardMacros.DoOnce` false :!label _label_2
    (:`Completed`
      (bind (_direction _newtrack_0) (`Timeline|Timeline_1` :!via `PlayFromStart`)
        (:`Update`
          (`SceneComponent.K2_SetRelativeLocation` (`self.DoorDown`) (`KismetMathLibrary.VLerp` (`SceneComponent.RelativeLocation` (`self.DoorDown`)) (`SceneComponent.RelativeLocation` (`self.doorDownP`)) _newtrack_0) false false))
        (:`Finished`
          (goto _label :!via `Reset`))))))

(fn `UserConstructionScript`)